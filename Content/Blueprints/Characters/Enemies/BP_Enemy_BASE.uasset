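; BP_Enemy_BASE is the base enemy Blueprint, handling defeat and removal from the level.
; On BeginPlay it binds to the Defeated event and destroys the actor when that fires.
; The Destroyed event spawns a destruction VFX actor at the enemy's location and rotation, so the effect follows any destruction.
; A TurnCharacter function flips the actor with a 180-degree rotation.
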(event `self.ReceiveBeginPlay`
  (`parent.ReceiveBeginPlay`)
  (add `self.Defeated` (delegate `OnDefeated`)))

(event `OnDefeated`
  (`self.K2_DestroyActor`))

(event `self.ReceiveDestroyed`
  (`|SpawnActorFromClass` "/Game/Blueprints/VFX/EnemyDestroyed/BP_VFX_Enemy_Destroyed.BP_VFX_Enemy_Destroyed_C" (`KismetMathLibrary.MakeTransform` (`self.K2_GetActorLocation`) (`self.K2_GetActorRotation`)) "AlwaysSpawn" "MultiplyWithRoot" null null))

(fn `TurnCharacter`
  (`self.K2_SetActorRotation` (`KismetMathLibrary.ComposeRotators` (`self.K2_GetActorRotation`) (struct :`Yaw` 180.0))))

(fn `UserConstructionScript`
  (`parent.UserConstructionScript`))